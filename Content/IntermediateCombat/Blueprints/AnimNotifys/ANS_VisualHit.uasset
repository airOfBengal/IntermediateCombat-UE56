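; Anim notify state that shows a visual hit effect on the animated mesh for the span of the notify.
; On begin it sets the materials' Hit scalar on and pushes its Color variable to the Color vector parameter; on end it clears Hit and writes the same Color again.
; When UseTyrant is set, it also sends the mesh owner an INTTyrantTimeMessage, true at begin and false at end.
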(fn `Received_NotifyBegin`
  (params (MeshComp :type "SkeletalMeshComponent Object Reference") (Animation :type "AnimSequenceBase Object Reference") (TotalDuration :type "Float (single-precision)") (EventReference :type "AnimNotifyEventReference Structure (by ref)"))
  (returns (ReturnValue :type Boolean))
  (bind (_color_r _color_g _color_b) (break `LinearColor` (`self.Color`)))
  (`MeshComponent.SetScalarParameterValueOnMaterials` MeshComp "Hit" 1.0)
  (`MeshComponent.SetVectorParameterValueOnMaterials` MeshComp "Color" (`KismetMathLibrary.MakeVector` _color_r _color_g _color_b))
  (if (`self.UseTyrant?`)
    (message `/Game/IntermediateCombat/Blueprints/Interfaces/BPI_Combat.INT_TyrantTime` (`ActorComponent.GetOwner` MeshComp) true)
    (return true)))

(fn `Received_NotifyEnd`
  (params (MeshComp :type "SkeletalMeshComponent Object Reference") (Animation :type "AnimSequenceBase Object Reference") (EventReference :type "AnimNotifyEventReference Structure (by ref)"))
  (returns (ReturnValue :type Boolean))
  (bind (_color_r _color_g _color_b) (break `LinearColor` (`self.Color`)))
  (`MeshComponent.SetScalarParameterValueOnMaterials` MeshComp "Hit" 0.0)
  (`MeshComponent.SetVectorParameterValueOnMaterials` MeshComp "Color" (`KismetMathLibrary.MakeVector` _color_r _color_g _color_b))
  (if (`self.UseTyrant?`)
    (message `/Game/IntermediateCombat/Blueprints/Interfaces/BPI_Combat.INT_TyrantTime` (`ActorComponent.GetOwner` MeshComp) false)
    (return true)))