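; BPC_Value is a component that tracks a clamped combat stat for its owner, either a depleting value or a posture bar that fills from zero.
; A looping timer applies the recovery amount and calls OnUpdateBars until the value reaches its limit.
; AddValue clamps changes, and an adverse one stops recovery and schedules it to resume after a delay, unless the bar has hit its breaking limit.
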(event `self.ReceiveBeginPlay`
  ;[0 0 0] Stats Recovery Logic
  (set `self.Owner` (`self.GetOwner`) :!label _label)
  (set `self.CurrentValue` (select `bool` (`self.PostureBar?`) :`false` (`self.MaxValue`)))
  (`self.Reco`))

(event `ReInitialize`
  ;[0 0 0] Stats Recovery Logic
  (goto _label))

(event `Reco`
  ;[0 0 0] Stats Recovery Logic
  (if (<= (`self.CurrentValue`) (`self.MaxValue`))
    (bind _returnvalue (`KismetSystemLibrary.K2_SetTimerDelegate` (delegate `Recovery`) 0.1 true)) ; Auto recovery
    (set `self.PropertyHandle` _returnvalue)))

(event `Recovery`
  (bind _propertyhandle (`self.PropertyHandle`))
  ;[0 0 0] Stats Recovery Logic
  (if (select `bool` (`self.PostureBar?`) :`false` (< (`self.CurrentValue`) (`self.MaxValue`)) :`true` (> (`self.CurrentValue`) 0.0))
    (set `self.CurrentValue` (`KismetMathLibrary.FClamp` (+ (`self.CurrentValue`) (`self.CurrentRecoveryValue`)) 0.0 (`self.MaxValue`)))
    (`self.OnUpdateBars`)
    (elif (`KismetSystemLibrary.K2_IsValidTimerHandle` _propertyhandle)
      (`KismetSystemLibrary.K2_ClearAndInvalidateTimerHandle` _propertyhandle))))

(event `ClearTimers`
  ;[0 0 0] Clear timers when value updated
  (`KismetSystemLibrary.K2_ClearAndInvalidateTimerHandle` (`self.PropertyHandle`))
  (`KismetSystemLibrary.K2_ClearAndInvalidateTimerHandle` (`self.StopHandle`)))

(fn `AddValue`
  (params (Added :type "Float (double-precision)"))
  (returns (CurrentValue :type "Float (double-precision)"))
  (bind _maxvalue (`self.MaxValue`))
  (bind _added (`local.Added`))
  (bind _output_get (set `self.CurrentValue` (`KismetMathLibrary.FClamp` (+ Added (`self.CurrentValue`)) 0.0 _maxvalue)))
  (if (select `bool` (`self.PostureBar?`) :`false` (< _output_get 0.1) :`true` (> _output_get (- _maxvalue 0.1)))
    (return (`self.CurrentValue`))
    (elif (select `bool` (`self.PostureBar?`) :`false` (< _added 0.0) :`true` (> _added 0.0))
      (`KismetSystemLibrary.K2_ClearAndInvalidateTimerHandle` (`self.PropertyHandle`))
      (bind _returnvalue (`KismetSystemLibrary.K2_SetTimer` null "Reco" 3.0)) ; Start to recover after 3 seconds
      (set `self.StopHandle` _returnvalue)
      (return (`self.CurrentValue`))
      (else
        (return (`self.CurrentValue`))))))

(fn `GetCurrentValue`
  (returns (CurrentValue :type "Float (double-precision)"))
  (return (`self.CurrentValue`)))