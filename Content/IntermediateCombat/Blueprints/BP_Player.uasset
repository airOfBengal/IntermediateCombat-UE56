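; Player pawn that handles movement and camera look for both PC and mobile, switched by a Mobile flag.
; BeginPlay activates the joystick touch interface for mobile after a short delay, and axis inputs drive movement relative to control rotation.
; A macro gates look input: axes rotate the camera on PC, while touch-drag deltas scaled by sensitivity rotate it on mobile.
; The construction script drops the mesh to the capsule's bottom.
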(event `self.ReceiveBeginPlay`
  (bind _aspc_in_game (cast `/Game/IntermediateCombat/Blueprints/System/PC_InGame` (`GameplayStatics.GetPlayerController` 0)))
  (bind _output_get (set `self.PC In Game` _aspc_in_game))
  (`KismetSystemLibrary.Delay` 0.2) ; A bit delay for initialization
  (`PlayerController.ActivateTouchInterface` _output_get (select `bool` (`self.Mobile?`) :`true` "/Game/IntermediateCombat/Blueprints/Misc/IC_Joysticks.IC_Joysticks" :!type "TouchInterface Object Reference")))

(event `InputAxis|MoveForward`
  (params (AxisValue :type "Float (single-precision)"))
  ; PC - Movement Control
  (`self.AddMovementInput` (`KismetMathLibrary.GetForwardVector` (`self.GetControlRotation`)) AxisValue))

(event `InputAxis|Turn`
  (params (AxisValue :type "Float (single-precision)"))
  ; PC - Camera rotation control
  (`self.CanRotateCameraInMobileMode`
    (:`false`
      (`self.AddControllerYawInput` AxisValue))))

(event `InputAxis|LookUp`
  (params (AxisValue :type "Float (single-precision)"))
  ; PC - Camera rotation control
  (`self.CanRotateCameraInMobileMode`
    (:`false`
      (`self.AddControllerPitchInput` AxisValue))))

(event `InputAxis|MoveRight`
  (params (AxisValue :type "Float (single-precision)"))
  ; PC - Movement Control
  (`self.AddMovementInput` (`KismetMathLibrary.GetRightVector` (`self.GetControlRotation`)) AxisValue))

(event `InputTouch`
  (params (Location :type "Vector Structure") (FingerIndex :type "ETouchIndex Enum"))
  (bind _x (.x Location))
  (bind _y (.y Location))
  ; Mobile - Camera rotation control
  (:`Pressed`
    (`self.CanRotateCameraInMobileMode` :!label _label
      (:`true`
        (set `self.YawVal` _x :!label _label_2)
        (set `self.PitchVal` _y))))
  (:`Released`
    (goto _label))
  (:`Moved`
    (`self.CanRotateCameraInMobileMode`
      (:`true`
        (`self.AddControllerYawInput` (/ (- _x (`self.YawVal`)) 6.0))
        (`self.AddControllerPitchInput` (/ (- _y (`self.PitchVal`)) 6.0))
        (goto _label_2)))))

(fn `UserConstructionScript`
  (`SceneComponent.K2_SetRelativeLocation` (`self.Mesh`) (`KismetMathLibrary.MakeVector` 0.0 0.0 (- 0.0 (`CapsuleComponent.GetUnscaledCapsuleHalfHeight` (`self.CapsuleComponent`)))) false false))