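; BP_Trainer is the AI sparring enemy for combat training, tuning attack counts, strafe timing and posture to the selected training mode.
; It runs BT_Trainer, strafes facing the player and deals damage through weapon overlaps or sphere traces.
; Hits drain HP and build posture, scaled by facing-based blocking, leading to stun or death.
; It also handles player deflects, jump hits, executions and hit-stop via brief time dilation.
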(fn `AddContinuousHitCounts`
  (bind _continuousattacked (`self.ContinuousAttacked`))
  (if (not (== _continuousattacked 3))
    (`/Engine/EditorBlueprintResources/StandardMacros.IncrementInt` _continuousattacked)))

(fn `INT_GetBlock`
  (returns (Block :type Boolean))
  (return false))

(fn `INT_GetDead`
  (returns (Dead :type Boolean))
  (return (`self.Dead`)))

(fn `INT_GetStun`
  (returns (`Stun?` :type Boolean))
  (return (and (not (`self.Dead`)) (`self.Stun`))))

(fn `ModesSelection`
  (bind _bpc_pb (`self.BPC_PB`))
  (bind _bpc_pb_2 (`self.BPC_PB`))
  (bind _asgi_ic (cast `/Game/IntermediateCombat/Blueprints/System/GI_IC` (`GameplayStatics.GetGameInstance`)))
  (switch `/Game/IntermediateCombat/Blueprints/Misc/Enums/E_TrainingModes` (`/Game/IntermediateCombat/Blueprints/System/GI_IC.TrainingMode` _asgi_ic) ; Preset parameters according to specified mode
    (:`NewEnumerator0`
      (set `self.InitAttackCounts` 0)
      (set `self.RechargeAtkCounts` 0)
      (bind _output_get (set `self.StrafeMinTime` 99999.0))
      (set `self.StrafeMaxTime` _output_get))
    (:`NewEnumerator1`
      (set `self.InitAttackCounts` 10 :!label _label)
      (set `self.RechargeAtkCounts` 10)
      (set `self.StrafeMinTime` 3.0)
      (set `self.StrafeMaxTime` 5.0)
      (set `/Game/IntermediateCombat/Blueprints/BPC/BPC_Value.MaxValue` 20.0 _bpc_pb) ; For player training
      (`/Game/IntermediateCombat/Blueprints/BPC/BPC_Value.ReInitialize` _bpc_pb :!label _label_2))
    (:`NewEnumerator2`
      (goto _label))
    (:`NewEnumerator3`
      (set `self.InitAttackCounts` 10)
      (set `self.RechargeAtkCounts` 10)
      (set `self.StrafeMinTime` 3.0)
      (set `self.StrafeMaxTime` 5.0)
      (set `/Game/IntermediateCombat/Blueprints/BPC/BPC_Value.MaxValue` 20.0 _bpc_pb) ; For player training
      (goto _label_2))
    (:`NewEnumerator4`
      (set `self.InitAttackCounts` 1)
      (set `self.RechargeAtkCounts` 4)
      (set `self.StrafeMinTime` 3.0)
      (set `self.StrafeMaxTime` 5.0)
      (set `/Game/IntermediateCombat/Blueprints/BPC/BPC_Value.MaxValue` 120.0 _bpc_pb) ; For player training
      (goto _label_2))
    (:`NewEnumerator5`
      (set `self.InitAttackCounts` 10)
      (set `self.RechargeAtkCounts` 10)
      (set `self.StrafeMinTime` 3.0)
      (set `self.StrafeMaxTime` 5.0)
      (set `/Game/IntermediateCombat/Blueprints/BPC/BPC_Value.MaxValue` 5.0 _bpc_pb) ; For player training
      (goto _label_2))
    (:`NewEnumerator6`
      (set `self.InitAttackCounts` 10)
      (set `self.RechargeAtkCounts` 10)
      (set `self.StrafeMinTime` 3.0)
      (set `self.StrafeMaxTime` 5.0)
      (set `/Game/IntermediateCombat/Blueprints/BPC/BPC_Value.MaxValue` 120.0 _bpc_pb) ; For player training
      (goto _label_2))
    (:`NewEnumerator7`
      (set `self.InitAttackCounts` 10)
      (set `self.RechargeAtkCounts` 10)
      (set `self.StrafeMinTime` 3.0)
      (set `self.StrafeMaxTime` 5.0)
      (set `/Game/IntermediateCombat/Blueprints/BP_Player.Enable Mikiri` true (`self.Target`)))
    (:`NewEnumerator8`
      (set `self.InitAttackCounts` 2)
      (set `self.RechargeAtkCounts` 3)
      (set `self.StrafeMinTime` 3.0)
      (set `self.StrafeMaxTime` 5.0)
      (set `/Game/IntermediateCombat/Blueprints/BP_Player.Enable Mikiri` true (`self.Target`))
      (set `/Game/IntermediateCombat/Blueprints/BPC/BPC_Value.MaxValue` 180.0 _bpc_pb_2) ; For player training
      (`/Game/IntermediateCombat/Blueprints/BPC/BPC_Value.ReInitialize` _bpc_pb_2))))

(fn `OnRep_Stun`
  ;[0 0 0] If AI is already in stun state, play sound
  (if (and (not (`self.Dead`)) (not (`self.Stun`)))
    (`/Game/IntermediateCombat/Blueprints/BPC/BPC_Value.Reco` (`self.BPC_PB`))
    (else
      (`GameplayStatics.SpawnSoundAtLocation` "/Game/IntermediateCombat/Demo/SFX/Cue_PoiseBreak.Cue_PoiseBreak" (`self.K2_GetActorLocation`) (struct) 1.0 1.0 0.8 null null))))

(fn `PostInitialization`
  (bind _asaic_dummy (cast `/Game/IntermediateCombat/Blueprints/AI/AIC_Dummy` (`AIBlueprintHelperLibrary.GetAIController` self)))
  (bind _output_get (set `self.AIC_Dummy` _asaic_dummy))
  (`AIController.RunBehaviorTree` _output_get "/Game/IntermediateCombat/Blueprints/AI/BT_Trainer.BT_Trainer")
  (set `self.Blackboard` (`AIController.Blackboard` _output_get)))

(fn `PreInitialization`
  (bind _asui_head_bar (cast `/Game/IntermediateCombat/Blueprints/UI/UI_HeadBar` (`WidgetComponent.GetUserWidgetObject` (`self.HeadBar`))))
  (set `self.UI_HeadBar` _asui_head_bar)
  (bind _asbp_player (cast `/Game/IntermediateCombat/Blueprints/BP_Player` (`GameplayStatics.GetPlayerCharacter` 0)))
  (set `self.Target` _asbp_player)
  (`self.UpdateHeadBar`)
  (`SceneComponent.SetHiddenInGame` (`self.HeadBar`) false false))

(fn `RecoverStun`
  (bind _returnvalue (`SkeletalMeshComponent.GetAnimInstance` (`self.Mesh`)))
  (`AnimInstance.Montage_Stop` _returnvalue 0.2 (`AnimInstance.GetCurrentActiveMontage` _returnvalue))
  (set `self.Stun` false) ; Start to recover
)

(fn `SelectFinalDamage`
  (params (AtkName :type "Array of String"))
  (switch `string` (`|GetArrayItem` AtkName)
    (:`00`
      (set `self.HPDamage` 80.0))
    (:`01`
      (set `self.HPDamage` 40.0))
    (:`02`
      (set `self.HPDamage` 60.0))
    (:`03`
      (set `self.HPDamage` 40.0))
    (:`04`
      (set `self.HPDamage` 60.0))))

(fn `TurnInPlaceAnim`
  (locals (L_RelativeRotation :type "Float (double-precision)"))
  (bind (_returnvalue_roll _returnvalue_pitch _returnvalue_yaw) (`KismetMathLibrary.BreakRotator` (`self.K2_GetActorRotation`)))
  (bind _l_relativerotation (`local.L_RelativeRotation`))
  (bind _target (`self.Target`)
    (:`then`
      (bind (_returnvalue_roll_2 _returnvalue_pitch_2 _returnvalue_yaw_2) (`KismetMathLibrary.BreakRotator` (`KismetMathLibrary.FindLookAtRotation` (`self.K2_GetActorLocation`) (`self.K2_GetActorLocation` _target))))
      (bind _output_get (set `local.L_RelativeRotation` (- _returnvalue_yaw_2 _returnvalue_yaw))) ; Whether player is within -30 ~ 30 degrees of trainer's front
      (if (not (or (and (> _output_get 0.0) (<= _output_get 30.0)) (and (> _output_get -360.0) (<= _output_get -330.0)) (and (> _output_get -30.0) (<= _output_get 0.0)) (and (> _output_get 330.0) (<= _output_get 360.0))))
        (`self.PlayAnimMontage` (select `bool` (or (and (> _l_relativerotation 0.0) (<= _l_relativerotation 180.0)) (and (> _l_relativerotation -360.0) (<= _l_relativerotation -180.0))) :`false` "/Game/IntermediateCombat/Animations/Montages/Tr_Turn_Left_90_Montage.Tr_Turn_Left_90_Montage" :`true` "/Game/IntermediateCombat/Animations/Montages/Tr_Turn_Right_90_Montage.Tr_Turn_Right_90_Montage" :!type "AnimMontage Object Reference"))))
    (:`else`)))

(fn `UpdateHeadBar`
  (bind _bpc_hp (`self.BPC_HP`))
  (bind _bpc_pb (`self.BPC_PB`))
  (bind _currentvalue (`/Game/IntermediateCombat/Blueprints/BPC/BPC_Value.GetCurrentValue` _bpc_hp))
  (bind _maxvalue (`/Game/IntermediateCombat/Blueprints/BPC/BPC_Value.MaxValue` _bpc_pb))
  (bind _ui_headbar (`self.UI_HeadBar`)
    (:`then`
      (`/Game/IntermediateCombat/Blueprints/UI/UI_HeadBar.UpdateHP` _ui_headbar _currentvalue (`/Game/IntermediateCombat/Blueprints/BPC/BPC_Value.MaxValue` _bpc_hp))
      (`/Game/IntermediateCombat/Blueprints/UI/UI_HeadBar.UpdatePB` _ui_headbar (`/Game/IntermediateCombat/Blueprints/BPC/BPC_Value.GetCurrentValue` _bpc_pb) _maxvalue)
      ;[0 0 0] Slow reocvery rate when HP is low
      (set `/Game/IntermediateCombat/Blueprints/BPC/BPC_Value.CurrentRecoveryValue` (`KismetMathLibrary.MapRangeClamped` _currentvalue _maxvalue 0.0 -2.5) (`self.BPC_PB`)))
    (:`else`)))

(fn `UserConstructionScript`
  (`SceneComponent.K2_SetRelativeLocation` (`self.Mesh`) (`KismetMathLibrary.MakeVector` 0.0 0.0 (- 0.0 (`CapsuleComponent.GetScaledCapsuleHalfHeight` (`self.CapsuleComponent`)))) false false))